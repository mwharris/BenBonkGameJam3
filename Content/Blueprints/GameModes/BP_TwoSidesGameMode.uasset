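; Game mode Blueprint for TwoSides that manages the HUD, the game-over screen and top-score persistence.
; On BeginPlay it creates the HUD and loads TopScore from a save slot, creating an empty save if none exists.
; NotifyUI events push score and player ship health to the HUD, or show game over with cursor and UI-only input.
; EndPlay saves TopScore, which is not calculated in this graph.
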(event EventBeginPlay
  (Input|SetInputModeGameOnly (Game|GetPlayerController 0))
  (bind _returnvalue (UserInterface|CreateWidget "/Game/UI/WBP_HUD.WBP_HUD_C"))
  (bind _output_get (Variables|Default|SetHUDRef _returnvalue))
  (UserInterface|Viewport|AddtoViewport _output_get 0)
  (CallFunction|LoadScore)
  (CallFunction|UpdateScore))

(event EventEndPlay
  (params (EndPlayReason :type EEndPlayReason%20Enum :default "Destroyed"))
  (CallFunction|SaveScore))

(event EventNotifyUIUpdateScore
  (CallFunction|UpdateScore))

(event EventNotifyUIUpdateHealth
  (bind _playership (Variables|Default|GetPlayerShip))
  (Default|UpdateHealth (Variables|Default|GetHUDRef) (Class|PawnBase|GetHealth _playership) (Class|PawnBase|GetMaxHealth _playership)))

(event EventNotifyUIGameOver
  (bind _returnvalue (Game|GetPlayerController 0))
  (bind _returnvalue_2 (UserInterface|CreateWidget "/Game/UI/WBP_GameOver.WBP_GameOver_C"))
  (UserInterface|Viewport|AddtoViewport _returnvalue_2 0)
  (Variables|/Script/Engine.PlayerController|SetbShowMouseCursor _returnvalue true)
  (Input|SetInputModeUIOnly _returnvalue 0 "DoNotLock"))

(fn ConstructionScript)

(fn LoadScore
  ;[1 1 1] Attempt to load saved Top Score
  (bind _returnvalue (SaveGame|LoadGamefromSlot (Variables|Default|GetSaveSlotName)))
  (Utilities|IsValid _returnvalue
    (:Is%20Valid
      ;[1 1 1] Load success, update our Top Score
      (bind _asbp_save_game (Utilities|Casting|CastToBP_SaveGame _returnvalue))
      (bind _output_get (Variables|Default|SetSaveGameData _asbp_save_game))
      (Variables|Default|SetTopScore (Variables|/Game/Blueprints/General/BP_SaveGame.BP_SaveGame_C|GetTopScore _output_get)))
    (:Is%20Not%20Valid
      ;[1 1 1] Load failed, create empty Save Game
      (bind _returnvalue_2 (SaveGame|CreateSaveGameObject "/Game/Blueprints/General/BP_SaveGame.BP_SaveGame_C"))
      (bind _output_get_2 (Variables|Default|SetSaveGameData _returnvalue_2))
      (SaveGame|SaveGametoSlot _output_get_2 (Variables|Default|GetSaveSlotName)))))

(fn SaveScore
  (bind _savegamedata (Variables|Default|GetSaveGameData))
  (Variables|/Game/Blueprints/General/BP_SaveGame.BP_SaveGame_C|SetTopScore _savegamedata (Variables|Default|GetTopScore))
  (SaveGame|SaveGametoSlot _savegamedata (Variables|Default|GetSaveSlotName)))

(fn UpdateScore
  (Default|UpdateScore (Variables|Default|GetHUDRef) (Class|TwoSidesGameMode|GetScore) (Variables|Default|GetTopScore)))