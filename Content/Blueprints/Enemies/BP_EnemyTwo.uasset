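; BP_EnemyTwo is an enemy ship Blueprint that makes a short scripted entry before enabling its movement.
; After the parent BeginPlay, a timeline lerps the actor from SpawnLocation along negative X using its EntrySpeed track, without sweeping.
; When the timeline finishes, it sets MoveEnabled to true.
; The construction script applies the Scale variable to the ship mesh's world scale.
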(event EventBeginPlay
  (bind _spawnlocation (Variables|Default|GetSpawnLocation))
  (|CallParentFunction)
  (bind _entryspeed (Timeline|Timeline_0 Play)
    (:Update
      (Transformation|SetActorLocation (Math|Vector|Lerp(Vector) _spawnlocation (- _spawnlocation "120.000000, 0,0.000000") _entryspeed) false false))
    (:Finished
      (Variables|Default|SetMoveEnabled true))))

(fn ConstructionScript
  (Transformation|SetWorldScale3D (Variables|Default|GetShipMesh) (Variables|Default|GetScale)))